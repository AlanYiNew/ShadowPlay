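; Lobby game mode that manages joining, leaving, kicking and character swaps, and server-travels to the selected arena.
; PostLogin registers each controller, initializes its lobby UI and possesses a default paper character at a random PlayerStart.
; EveryoneUpdate rebuilds the player list, pushes it with available characters to all controllers, and derives CanWeStart from status text and chosen pawn.
; Map setting changes are relayed to every stored controller.
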(event `self.K2_OnLogout`
  (params (ExitingController :type "Controller Object Reference"))
  ;[1 1 1] On Logout of player
  (`/Engine/EditorBlueprintResources/ActorMacros.Switch Has Authority`
    (:`Authority`
      (bind _asbp_lobby_player_controller (cast `/Game/Lobby/BP_LobbyPlayerController` ExitingController))
      (`KismetArrayLibrary.Array_RemoveItem` (`self.AllLobbyControllers`) _asbp_lobby_player_controller)
      (`self.EveryoneUpdate`))))

(event `self.K2_PostLogin`
  (params (NewPlayer :type "PlayerController Object Reference"))
  ;[1 1 1] Initial Setup Occurs on PostLogin Event - Handle Lobby Settup On Player Controller and spawn player
  (`/Engine/EditorBlueprintResources/ActorMacros.Switch Has Authority`
    (:`Authority`
      (`KismetArrayLibrary.Array_Add` (`self.AllLobbyControllers`) NewPlayer)
      (bind _outactors (`GameplayStatics.GetAllActorsOfClass` "/Script/Engine.PlayerStart"))
      (set `self.Spawn Points` _outactors)
      (bind _asmy_game_instance (cast `/Game/AllLevel/MyGameInstance` (`GameplayStatics.GetGameInstance`)))
      (set `self.ServerName` (`/Game/AllLevel/MyGameInstance.Server Name` _asmy_game_instance))
      (set `self.MaxPlayer` (`/Game/AllLevel/MyGameInstance.MaxPlayer` _asmy_game_instance))
      (bind _asbp_lobby_player_controller (cast `/Game/Lobby/BP_LobbyPlayerController` NewPlayer))
      (`/Game/Lobby/BP_LobbyPlayerController.InitilizeSetup` _asbp_lobby_player_controller)
      (`/Game/Lobby/BP_LobbyPlayerController.SetupLobbyMenu` _asbp_lobby_player_controller (`self.ServerName`))
      (`/Game/Lobby/BP_LobbyPlayerController.UpdateLobbySetting` _asbp_lobby_player_controller (`self.GM_MapImage`) (`self.GM_MapName`) (`self.GM_MapTime`))
      (`self.RespawnPlayer` NewPlayer))))

(event `ServerUpdateGameSettings`
  (params (NewImage :type "Texture2D Object Reference") (MapName :type Text) (MapTime :type Text) (MapID :type Integer))
  ;[1 1 1] Server has made changes / tell each client to update lobby information
  (set `self.GM_MapImage` NewImage)
  (set `self.GM_MapName` MapName)
  (set `self.GM_MapTime` MapTime)
  (set `self.GM_MapID` MapID)
  (for _array_element (`self.AllLobbyControllers`)
    (bind _asbp_lobby_player_controller (cast `/Game/Lobby/BP_LobbyPlayerController` _array_element))
    (`/Game/Lobby/BP_LobbyPlayerController.UpdateLobbySetting` _asbp_lobby_player_controller (`self.GM_MapImage`) (`self.GM_MapName`) (`self.GM_MapTime`))))

(event `RespawnPlayer`
  (params (PlayerController :type "PlayerController Object Reference"))
  (bind _returnvalue (`Controller.K2_GetPawn` PlayerController))
  ;[1 1 1] Spawn the pawn as base character when arriving Lobby / Tells everyone to update their lobby
  (`/Engine/EditorBlueprintResources/StandardMacros.IsValid` _returnvalue
    (:`Is Valid`
      (`self.K2_DestroyActor` _returnvalue))
    (:`Is Not Valid`
      _))
  (bind _transform (`self.GetSpawnPoint`))
  (bind _returnvalue_2 (`|SpawnActorFromClass` "/Game/Characters/BlankCharacter/BP_DefaultPaperCharacter.BP_DefaultPaperCharacter_C" _transform "Undefined" "OverrideRootScale" null null))
  (`Controller.Possess` PlayerController _returnvalue_2)
  (`self.EveryoneUpdate`))

(event `LaunchTheGame`
  (bind _returnvalue (`GameplayStatics.GetPlayerController` 0))
  ;[1 1 1] Launch game based on map selected from game settings
  (switch `int` (`self.GM_MapID`)
    (:`0`
      (`KismetSystemLibrary.ExecuteConsoleCommand` "servertravel/Game/Maps/Arena01" _returnvalue))
    (:`1`
      (`KismetSystemLibrary.ExecuteConsoleCommand` "servertravel/Game/Maps/Arena02" _returnvalue))))

(event `EveryoneUpdate`
  (bind _alllobbycontrollers (`self.AllLobbyControllers`))
  (bind _connectedplayers (`self.ConnectedPlayers`))
  ;[1 1 1] Update All Connected Player' Lobby Information when called
  (bind _output_get (set `self.CurrentPlayers` (`KismetArrayLibrary.Array_Length` (`self.AllLobbyControllers`))))
  (if (> _output_get 0)
    (`KismetArrayLibrary.Array_Clear` (`self.ConnectedPlayers`))
    (for _array_element _alllobbycontrollers
      (bind _asbp_lobby_player_controller (cast `/Game/Lobby/BP_LobbyPlayerController` _array_element))
      (bind _structout (setmembers `/Game/AllLevel/PlayerInfo` :`StructRef` (`/Game/Lobby/BP_LobbyPlayerController.PlayerSetttings` _asbp_lobby_player_controller) :`IsServer` (and (`|EnumEquality` (`self.GetRemoteRole` _asbp_lobby_player_controller) "ROLE_SimulatedProxy") (`|EnumEquality` (`self.GetLocalRole` _asbp_lobby_player_controller) "ROLE_Authority")) :`PlayerIndex` (`KismetArrayLibrary.Array_Length` _connectedplayers)))
      (`KismetArrayLibrary.Array_Add` _connectedplayers _structout)
      (`/Game/Lobby/BP_LobbyPlayerController.UpdateNumberOfPlayers` _asbp_lobby_player_controller (`self.CurrentPlayers`) (`self.MaxPlayer`)))
    (for _array_element_2 _alllobbycontrollers
      (bind _asbp_lobby_player_controller_2 (cast `/Game/Lobby/BP_LobbyPlayerController` _array_element_2))
      (`/Game/Lobby/BP_LobbyPlayerController.AddPlayerInfo` _asbp_lobby_player_controller_2 (`self.ConnectedPlayers`))
      (`/Game/Lobby/BP_LobbyPlayerController.UpdateAvailableCharacter` _asbp_lobby_player_controller_2 (`self.Available Charcters`)))
    (for _array_element_3 (`self.ConnectedPlayers`) :!label _label
      (bind _bool (`self.CanNotCheck` _array_element_3))
      (if _bool
        (set `self.CanWeStart` false)
        (`self.Can not start Game`)
        (else
          (set `self.CanWeStart` true))))))

(event `Can not start Game`
  ;[1 1 1] Update All Connected Player' Lobby Information when called
  (goto _label :!via `Break`))

(event `SwapCharacter`
  (params (PlayerController :type "PlayerController Object Reference") (PawnClass :type "Pawn Class Reference") (ChangedStatus :type Boolean))
  (bind _returnvalue (`Controller.K2_GetPawn` PlayerController))
  ;[1 1 1] Swap Character
  (if (not ChangedStatus)
    (`/Engine/EditorBlueprintResources/StandardMacros.IsValid` _returnvalue
      (:`Is Valid`
        (`self.K2_DestroyActor` _returnvalue))))
  (bind _transform (`self.GetSpawnPoint`))
  (bind _returnvalue_2 (`|SpawnActorFromClass` PawnClass _transform "Undefined" "OverrideRootScale" null null))
  (`Controller.Possess` PlayerController _returnvalue_2)
  (`self.EveryoneUpdate`))

(event `YouHaveBeenKicked`
  (params (PlayerID :type Integer))
  ;[1 1 1] Kick Selecetd Player
  (`/Game/Lobby/BP_LobbyPlayerController.Kicked` (cast `/Game/Lobby/BP_LobbyPlayerController` (`|GetArrayItem` (`self.AllLobbyControllers`) PlayerID) :!pure true)))

(fn `CanNotCheck`
  (params (PlayerInfo :type "/Game/AllLevel/PlayerInfo Structure"))
  (returns (bool :type Boolean))
  (bind (_myplayername _myplayercharacter _pawnclass _playerstatus) (break `/Game/AllLevel/PlayerInfo` PlayerInfo))
  (return (or (and (`KismetStringLibrary.NotEqual_StrStr` (`KismetTextLibrary.Conv_TextToString` _playerstatus) "房主") (`KismetStringLibrary.NotEqual_StrStr` (`KismetTextLibrary.Conv_TextToString` _playerstatus) "已准备")) (== _pawnclass "/Game/Characters/BlankCharacter/BP_DefaultPaperCharacter.BP_DefaultPaperCharacter_C"))))

(fn `GetSpawnPoint`
  (returns (Transform :type "Transform Structure"))
  (bind _spawn_points (`self.Spawn Points`))
  (return (`self.GetTransform` (`|GetArrayItem` _spawn_points (`KismetMathLibrary.RandomIntegerInRange` 0 (- (`KismetArrayLibrary.Array_Length` _spawn_points) 1))))))

(fn `NewFunction_0`
  (params (StructRef :type "/Game/AllLevel/PlayerInfo Structure (by ref)") (IsServer :type Boolean))
  (returns (StructOut :type "/Game/AllLevel/PlayerInfo Structure (by ref)"))
  (bind _structout (setmembers `/Game/AllLevel/PlayerInfo` :`StructRef` StructRef :`MyPlayerName` "" :`MyPlayerCharacter` "None" :`PawnClass` null :`PlayerStatus` "" :`MyCharacterImage` null :`IsServer` IsServer))
  (return _structout))

(fn `UserConstructionScript`)